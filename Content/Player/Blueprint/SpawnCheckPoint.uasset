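; SpawnCheckPoint is a checkpoint trigger that saves a respawn point when an actor tagged Player overlaps it.
; It plays the checkpoint sound at world origin and stores its root transform in the GM game instance.
; It then spawns a CheckPoints actor there, destroys itself, and removes the first CheckPoints actor found, falling back to the second if the first is invalid.
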(event `self.ReceiveActorBeginOverlap`
  (params (OtherActor :type "Actor Object Reference"))
  (bind _returnvalue (`SceneComponent.K2_GetComponentToWorld` (`self.DefaultSceneRoot`)))
  (if (`self.ActorHasTag` OtherActor "Player")
    (`GameplayStatics.SpawnSoundAtLocation` "/Game/Sounds/Checkpoint.Checkpoint")
    (bind _asgm (cast `/Game/Player/Blueprint/GM` (`GameplayStatics.GetGameInstance`)))
    (set `/Game/Player/Blueprint/GM.CheckPoint` _returnvalue _asgm)
    (`|SpawnActorFromClass` "/Game/Player/Blueprint/CheckPoints.CheckPoints_C" _returnvalue "Undefined" "OverrideRootScale")
    (`self.K2_DestroyActor`)
    (bind _outactors (`GameplayStatics.GetAllActorsOfClass` "/Game/Player/Blueprint/CheckPoints.CheckPoints_C"))
    (bind _output (`|GetArrayItem` _outactors))
    (`/Engine/EditorBlueprintResources/StandardMacros.IsValid` _output
      (:`Is Valid`
        (`self.K2_DestroyActor` _output))
      (:`Is Not Valid`
        (`self.K2_DestroyActor` (`|GetArrayItem` _outactors 1))))))

(fn `UserConstructionScript`)
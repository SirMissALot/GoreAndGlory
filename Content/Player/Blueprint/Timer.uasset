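; Timer is an actor that runs the game's countdown until the player wins.
; Each Tick, while the ThirdPersonCharacter's Win flag is false, it subtracts delta seconds from CurrentTime on the GM game instance and stores the truncated result as a Timespan.
; ReturnTime formats that Timespan as a minutes:seconds string without zero padding.
; The countdown has no check for reaching zero.
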(event `self.ReceiveTick`
  (params (DeltaSeconds :type "Float (single-precision)"))
  (bind _asthird_person_character (cast `/Game/Player/Blueprint/ThirdPersonCharacter` (`GameplayStatics.GetPlayerPawn` 0)))
  (if (not (`/Game/Player/Blueprint/ThirdPersonCharacter.Win` _asthird_person_character))
    (bind _asgm (cast `/Game/Player/Blueprint/GM` (`GameplayStatics.GetGameInstance`)))
    (bind _output_get (set `/Game/Player/Blueprint/GM.CurrentTime` (- (`/Game/Player/Blueprint/GM.CurrentTime` _asgm) DeltaSeconds) _asgm))
    (set `self.Time` (`KismetMathLibrary.MakeTimespan` 0 0 0 (`KismetMathLibrary.FTrunc` _output_get)))))

(fn `Return Time`
  (returns (Time :type String))
  (bind (_days _hours _minutes _seconds) (`KismetMathLibrary.BreakTimespan` (`self.Time`)))
  (return (`KismetStringLibrary.Concat_StrStr` (`KismetStringLibrary.Conv_IntToString` _minutes) ":" (`KismetStringLibrary.Conv_IntToString` _seconds))))

(fn `UserConstructionScript`)
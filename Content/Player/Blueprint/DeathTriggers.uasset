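; DeathTriggers is a trigger Blueprint that kills the player when they overlap it at speed.
; Overlap by a "Player"-tagged actor plays the Crash sound at world origin, whatever the speed.
; Above a velocity threshold, it increments DeathCount on the GM game instance and sets IsDead on the ThirdPersonCharacter.
; An alternative check using GetOverlappingActors is left unconnected, and Tick is empty.
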(event `self.ReceiveActorBeginOverlap`
  (params (OtherActor :type "Actor Object Reference"))
  ;[1 1 1] DeathCount+
  (if (`self.ActorHasTag` OtherActor "Player")
    (`GameplayStatics.SpawnSoundAtLocation` "/Game/Sounds/Crash.Crash")
    (if (> (`KismetMathLibrary.VSize` (`self.GetVelocity` OtherActor)) 200.0)
      (bind _asgm (cast `/Game/Player/Blueprint/GM` (`GameplayStatics.GetGameInstance`)))
      (set `/Game/Player/Blueprint/GM.DeathCount` (+ (`/Game/Player/Blueprint/GM.DeathCount` _asgm) 1) _asgm)
      (bind _asthird_person_character (cast `/Game/Player/Blueprint/ThirdPersonCharacter` OtherActor))
      (set `/Game/Player/Blueprint/ThirdPersonCharacter.IsDead` true _asthird_person_character))))

(event `self.ReceiveBeginPlay`)

(event `self.ReceiveTick`
  (params (DeltaSeconds :type "Float (single-precision)"))
  ;[1 1 1] Collision
)

(fn `UserConstructionScript`)
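; Laser death trigger actor that kills the player character on contact.
; On overlap with a Player-tagged actor, it plays a crash sound at world origin and, if that actor moves faster than a speed threshold, increments DeathCount on the GM game instance and sets IsDead.
; Separately, Tick polls the Capsule's first overlapping ThirdPersonCharacter and sets IsDead regardless of speed, without counting the death.
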(event `self.ReceiveActorBeginOverlap`
  (params (OtherActor :type "Actor Object Reference"))
  ;[1 1 1] DeathCount+
  (if (`self.ActorHasTag` OtherActor "Player")
    (`GameplayStatics.SpawnSoundAtLocation` "/Game/Sounds/Crash.Crash")
    (if (> (`KismetMathLibrary.VSize` (`self.GetVelocity` OtherActor)) 200.0)
      (bind _asgm (cast `/Game/Player/Blueprint/GM` (`GameplayStatics.GetGameInstance`)))
      (set `/Game/Player/Blueprint/GM.DeathCount` (+ (`/Game/Player/Blueprint/GM.DeathCount` _asgm) 1) _asgm)
      (bind _asthird_person_character (cast `/Game/Player/Blueprint/ThirdPersonCharacter` OtherActor))
      (set `/Game/Player/Blueprint/ThirdPersonCharacter.IsDead` true _asthird_person_character))))

(event `self.ReceiveBeginPlay`)

(event `self.ReceiveTick`
  (params (DeltaSeconds :type "Float (single-precision)"))
  (bind _output (`|GetArrayItem` (`PrimitiveComponent.GetOverlappingActors` (`self.Capsule`) "/Game/Player/Blueprint/ThirdPersonCharacter.ThirdPersonCharacter_C")))
  ;[1 1 1] Collision
  (`/Engine/EditorBlueprintResources/StandardMacros.IsValid` _output
    (:`Is Valid`
      (bind _asthird_person_character (cast `/Game/Player/Blueprint/ThirdPersonCharacter` _output))
      (set `/Game/Player/Blueprint/ThirdPersonCharacter.IsDead` true _asthird_person_character))))

(fn `UserConstructionScript`)
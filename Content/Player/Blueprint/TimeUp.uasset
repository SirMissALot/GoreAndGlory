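; Player-side time-up actor that ends play when the game timer runs out.
; Each tick it reads CurrentTime from the GM game instance and, once it reaches zero, fires a DoOnce.
; That disables the player's ThirdPersonCharacter, clears all widgets and shows the UI_TImeUp screen.
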(event `self.ReceiveTick`
  (params (DeltaSeconds :type "Float (single-precision)"))
  (bind _asgm (cast `/Game/Player/Blueprint/GM` (`GameplayStatics.GetGameInstance`)))
  (if (<= (`/Game/Player/Blueprint/GM.CurrentTime` _asgm) 0.0)
    (`/Engine/EditorBlueprintResources/StandardMacros.DoOnce` false
      (:`Completed`
        (bind _asthird_person_character (cast `/Game/Player/Blueprint/ThirdPersonCharacter` (`GameplayStatics.GetPlayerPawn` 0)))
        (set `/Game/Player/Blueprint/ThirdPersonCharacter.Disabled` true _asthird_person_character)
        (`WidgetLayoutLibrary.RemoveAllWidgets`)
        (bind _returnvalue (`|CreateWidget` "/Game/Widgets/UI_TImeUP.UI_TImeUp_C"))
        (`UserWidget.AddToViewport` _returnvalue 0)))))

(fn `UserConstructionScript`)
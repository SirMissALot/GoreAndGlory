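; Sphere_Blueprint is an actor that rocks back and forth around its local pitch axis.
; Each Tick it adds a local pitch step, using Start or End according to the ChangedRot flag.
; The flag flips when actor pitch passes a lower or upper limit, reversing the swing.
; The steps are not scaled by delta time, so the speed depends on frame rate.
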(event `self.ReceiveTick`
  (params (DeltaSeconds :type "Float (single-precision)"))
  (bind (_returnvalue_roll _returnvalue_pitch) (`KismetMathLibrary.BreakRotator` (`self.K2_GetActorRotation`)))
  (bind (_returnvalue_roll_2 _returnvalue_pitch_2) (`KismetMathLibrary.BreakRotator` (`self.K2_GetActorRotation`)))
  (if (`self.changedRot`)
    (`self.K2_AddActorLocalRotation` (`KismetMathLibrary.MakeRotator` 0.0 (`self.start`)))
    (if (<= _returnvalue_pitch -60.0)
      (set `self.changedRot` (not (`self.changedRot`)) :!label _label))
    (else
      (`self.K2_AddActorLocalRotation` (`KismetMathLibrary.MakeRotator` 0.0 (`self.end`)))
      (if (>= _returnvalue_pitch_2 60.0)
        (goto _label)))))

(fn `UserConstructionScript`)
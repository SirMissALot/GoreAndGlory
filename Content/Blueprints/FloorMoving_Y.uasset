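; FloorMoving_Y is a moving floor actor that shuttles back and forth between Start and End reference actors.
; Each Tick offsets it in local space by its Speed vector scaled by delta time, without sweep.
; The sign of Speed.Y selects the target, Start when positive and End otherwise.
; Coming within 50 units of that target negates the whole Speed vector to reverse travel.
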(event `self.ReceiveTick`
  (params (DeltaSeconds :type "Float (single-precision)"))
  (bind (_speed_x _speed_y) (`KismetMathLibrary.BreakVector` (`self.speed`)))
  (`self.K2_AddActorLocalOffset` (* (`self.speed`) DeltaSeconds))
  (if (> (`KismetMathLibrary.SignOfFloat` _speed_y) 0.0)
    (if (== (`self.K2_GetActorLocation`) (`self.K2_GetActorLocation` (`self.start`)) :`ErrorTolerance` 50.0)
      (set `self.speed` (* (`self.speed`) -1) :!label _label))
    (elif (== (`self.K2_GetActorLocation`) (`self.K2_GetActorLocation` (`self.end`)) :`ErrorTolerance` 50.0)
      (goto _label))))

(fn `UserConstructionScript`)
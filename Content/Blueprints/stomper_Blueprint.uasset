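; Stomper actor that oscillates between its spawn location and a referenced Start actor, likely as a crusher hazard.
; Tick moves it by a local Speed offset without sweep, using a Stomped flag to choose which endpoint to test.
; Near spawn it switches to Fastspeed, near Start to SlowSpeed, toggling the flag each time.
; A Delay called from Tick precedes the spawn-side check.
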(event `self.ReceiveBeginPlay`
  (set `self.end` (`self.K2_GetActorLocation`)))

(event `self.ReceiveTick`
  (params (DeltaSeconds :type "Float (single-precision)"))
  (`self.K2_AddActorLocalOffset` (* (`self.speed`) DeltaSeconds))
  (if (`self.stomped`)
    (`KismetSystemLibrary.Delay` (`self.delay`))
    (if (== (`self.K2_GetActorLocation`) (`self.end`) :`ErrorTolerance` 25.0)
      (set `self.speed` (`self.fastspeed`))
      (set `self.stomped` (not (`self.stomped`)) :!label _label))
    (elif (== (`self.K2_GetActorLocation`) (`self.K2_GetActorLocation` (`self.start`)) :`ErrorTolerance` 50.0)
      (set `self.speed` (`self.slowSpeed`))
      (goto _label))))

(fn `UserConstructionScript`)